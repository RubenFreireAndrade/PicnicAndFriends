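; Inventory component that stores items as stacks in a slot array, sized at BeginPlay, and toggles its inventory window.
; Adding finds a partial stack of the same class or fills an empty slot.
; Stacking sets the slot to max and recursively re-adds the remainder whenever the combined quantity exceeds zero, not max stack.
; InventoryQuery checks single slots for an item and amount; ToggleInventory centers the window on the HUD canvas and switches input mode.
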(event EventBeginPlay
  (CallFunction|PrepareInventory))

(event EventTick
  (params (DeltaSeconds :type Float%20%28single-precision%29)))

(fn ToggleInventory
  (bind _returnvalue (Game|GetPlayerController 0))
  (bind _returnvalue_2 (Game|GetPlayerController 0))
  (Variables|Default|GetInventoryWindow
    (:then
      (Widget|RemovefromParent (Variables|Default|GetInventoryWindow))
      (Variables|Default|SetInventoryWindow 0)
      (Input|SetInputModeGameOnly _returnvalue_2)
      (Variables|/Script/Engine.PlayerController|SetbShowMouseCursor _returnvalue_2 false))
    (:else
      (bind _returnvalue_3 (UserInterface|CreateWidget "/Game/MyBlueprints/Gameplay/InventorySystem/InventoryUI/InventoryWindow.InventoryWindow_C" 0 self))
      (Variables|Default|SetInventoryWindow _returnvalue_3)
      (bind _asbp_my_player_controller (Utilities|Casting|CastToBP_MyPlayerController (Game|GetPlayerController 0)))
      (bind _returnvalue_4 (Class|CanvasPanel|AddChildtoCanvas (Variables|/Game/MyBlueprints/Gameplay/InventorySystem/InventoryUI/HUD.HUD_C|GetHudCanvas (Variables|/Game/MyBlueprints/Gameplay/Player/BP_MyPlayerController.BP_MyPlayerController_C|GetHudWidget _asbp_my_player_controller)) (Variables|Default|GetInventoryWindow)))
      (Class|CanvasPanelSlot|SetAutoSize _returnvalue_4 true)
      (Class|CanvasPanelSlot|SetAlignment _returnvalue_4 "(X=0.500000,Y=0.500000)")
      (Class|CanvasPanelSlot|SetAnchors _returnvalue_4 (Utilities|Struct|MakeAnchors "(X=0.500000,Y=0.500000)" "(X=0.500000,Y=0.500000)"))
      (Class|CanvasPanelSlot|SetPosition _returnvalue_4 (Variables|Default|GetPosition))
      (Input|SetInputModeUIOnly _returnvalue (Variables|Default|GetInventoryWindow) "LockAlways")
      (Variables|/Script/Engine.PlayerController|SetbShowMouseCursor _returnvalue true))))

(fn AddtoInventory
  (params (ContentToAdd :type Slot%20Structure%20Structure))
  (if true
    (bind _stackindex (Utilities|HasPartialStack ContentToAdd)
      (:True
        (CallFunction|AddtoStack ContentToAdd _stackindex))
      (:False
        (CallFunction|CreateStack ContentToAdd :!label _label)))
    (else
      (goto _label)))
  (return true))

(fn PrepareInventory
  (Utilities|Array|Resize (Variables|Default|GetInventory) (Variables|Default|GetNumberOfSlots)))

(fn CreateStack
  (params (ContentToAdd :type Slot%20Structure%20Structure))
  (bind _inventory (Variables|Default|GetInventory))
  (Utilities|Array|SetArrayElem _inventory (Utilities|Array|FindItem _inventory (Utilities|Struct|MakeSlotStructure "(Name_2_E4FCCCF2415A7B880428568CE265F690=NSLOCTEXT(\"[212C611E4063DCDEF7B57583D9CD9BF2]\", \"E04F2E8742E7BCC94BEED4830519CFD4\", \"None\"),isStackable_7_62B26FAB4BC04A706C722797E3C992CE=True,thumbnail_9_67725CD9403BEA07F5C2CDA30062DCF3=None,Class_12_AF1AF12A4F0498BC96E161BF73632AA2=None,MaxStack_15_D7DF4220481B8B4473C4A2BEC01741EB=0)")) ContentToAdd))

(fn AddtoStack
  (params (Slot%20Structure :type Slot%20Structure%20Structure) (SlotIndex :type Integer))
  (bind _inventory (Variables|Default|GetInventory))
  (bind _maxstack (Utilities|Struct|BreakItemStructure (.itemstructure Slot%20Structure)))
  (bind _output (Utilities|Array|Get(acopy) _inventory SlotIndex))
  (bind _output_get (LocalVariables|SetCurrentQuantity (.quantity (Utilities|Array|Get(acopy) (Variables|Default|GetInventory) SlotIndex))))
  (if (> (+ _output_get (.quantity (Utilities|Struct|BreakSlotStructure Slot%20Structure))) 0)
    (Utilities|Array|SetArrayElem (Variables|Default|GetInventory) SlotIndex (Utilities|Struct|MakeSlotStructure (.itemstructure Slot%20Structure) _maxstack))
    (CallFunction|AddtoInventory (Utilities|Struct|MakeSlotStructure (.itemstructure Slot%20Structure) (- (.quantity Slot%20Structure) (- _maxstack (LocalVariables|GetCurrentQuantity)))))
    (else
      (Utilities|Array|SetArrayElem _inventory SlotIndex (Utilities|Struct|MakeSlotStructure (.itemstructure _output) (+ (.quantity _output) (.quantity Slot%20Structure))))))
  (return))

(fn InventoryQuery
  (params (QueryItem :type Item%20Class%20Reference) (QueryAmount :type Integer))
  (bind _array_element (Utilities|Array|ForEachLoopwithBreak (Variables|Default|GetInventory) :!label _label)
    (:LoopBody
      (bind _output_get (LocalVariables|SetSuccess (and (>= (.quantity _array_element) QueryAmount) (== (.Class (Utilities|Struct|BreakItemStructure (.itemstructure _array_element))) QueryItem))))
      (if _output_get
        (goto _label Break)))
    (:Completed
      (return (LocalVariables|GetSuccess)))))