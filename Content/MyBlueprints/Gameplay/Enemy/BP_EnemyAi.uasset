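; Enemy AI Blueprint that reports sightings to the seen pawn and chases it once detection is set.
; PawnSensing starts the pawn's detection message once, and a short retriggerable delay stops it and resets the gate when sightings cease.
; StartChase and StopChase toggle IsDetected, which gates AIMoveTo toward the seen pawn on each sighting.
; StopChase also issues a move to itself and prints a debug message.
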(event OnSeePawn(PawnSensing)
  (params (Pawn :type Pawn%20Object%20Reference))
  (bind _self self)
  (Utilities|FlowControl|Sequence
    (:then_0
      (Utilities|FlowControl|Sequence
        (:then_0
          (Utilities|FlowControl|DoOnce false :!label _label
            (:Completed
              (Class|DetectionInterface|StartDetection(Message) Pawn _self))))
        (:then_1
          (if (Variables|Default|GetIsDetected)
            (AI|AIMoveTo _self "0, 0, 0" Pawn 5.0 false)))))
    (:then_1
      (Utilities|FlowControl|RetriggerableDelay 0.5)
      (Class|DetectionInterface|StopDetection(Message) Pawn)
      (goto _label Reset))))

(event EventStopChase
  (bind _self self)
  (Variables|Default|SetIsDetected false)
  (AI|AIMoveTo _self "0, 0, 0" _self 5.0 false
    (:then
      (Development|PrintString "Stopped Chasing"))))

(event EventStartChase
  (Variables|Default|SetIsDetected true)
  (Development|PrintString "Detected"))

(fn ConstructionScript)