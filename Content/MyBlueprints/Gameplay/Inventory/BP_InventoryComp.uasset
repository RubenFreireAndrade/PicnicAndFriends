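; Actor component that gives its owner a fixed-size, slot-based inventory and a toggleable inventory window.
; BeginPlay sizes the slot array; ToggleInventory adds or removes a centred widget on the player controller's HUD canvas, switching input mode and cursor.
; CreateStack writes content into the first empty slot.
; Stacking is unfinished: HasPartialStack's comparisons are unwired, and AddToInventory's hard-coded condition never reaches CreateStack.
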(event EventBeginPlay
  (CallFunction|PrepareInventory))

(event EventTick
  (params (DeltaSeconds :type Float%20%28single-precision%29)))

(fn ToggleInventory
  (bind _returnvalue (Game|GetPlayerController 0))
  (bind _returnvalue_2 (Game|GetPlayerController 0))
  (Variables|Default|GetInventoryWindow
    (:then
      (Widget|RemovefromParent (Variables|Default|GetInventoryWindow))
      (Variables|Default|SetInventoryWindow 0)
      (Input|SetInputModeGameOnly _returnvalue_2)
      (Variables|/Script/Engine.PlayerController|SetbShowMouseCursor _returnvalue_2 false))
    (:else
      (bind _returnvalue_3 (UserInterface|CreateWidget "/Game/MyBlueprints/Gameplay/Inventory/InventoryUI/InventoryWindow.InventoryWindow_C" 0 self))
      (Variables|Default|SetInventoryWindow _returnvalue_3)
      (bind _asbp_my_player_controller (Utilities|Casting|CastToBP_MyPlayerController (Game|GetPlayerController 0)))
      (bind _returnvalue_4 (Class|CanvasPanel|AddChildtoCanvas (Variables|/Game/MyBlueprints/Gameplay/Inventory/InventoryUI/HUD.HUD_C|GetHudCanvas (Variables|/Game/MyBlueprints/Gameplay/BP_MyPlayerController.BP_MyPlayerController_C|GetHudWidget _asbp_my_player_controller)) (Variables|Default|GetInventoryWindow)))
      (Class|CanvasPanelSlot|SetAutoSize _returnvalue_4 true)
      (Class|CanvasPanelSlot|SetAlignment _returnvalue_4 "(X=0.500000,Y=0.500000)")
      (Class|CanvasPanelSlot|SetAnchors _returnvalue_4 (Utilities|Struct|MakeAnchors "(X=0.500000,Y=0.500000)" "(X=0.500000,Y=0.500000)"))
      (Class|CanvasPanelSlot|SetPosition _returnvalue_4 (Variables|Default|GetPosition))
      (Input|SetInputModeGameandUI _returnvalue (Variables|Default|GetInventoryWindow) "LockAlways" true)
      (Variables|/Script/Engine.PlayerController|SetbShowMouseCursor _returnvalue true))))

(fn AddtoInventory
  (params (ContentToAdd :type Slot%20Structure%20Structure))
  (if (not true)
    (CallFunction|CreateStack ContentToAdd)
    (return true)))

(fn PrepareInventory
  (Utilities|Array|Resize (Variables|Default|GetInventory) (Variables|Default|GetNumberOfSlots)))

(fn CreateStack
  (params (ContentToAdd :type Slot%20Structure%20Structure))
  (bind _inventory (Variables|Default|GetInventory))
  (Utilities|Array|SetArrayElem _inventory (Utilities|Array|FindItem _inventory (Utilities|Struct|MakeSlotStructure "(Name_2_E4FCCCF2415A7B880428568CE265F690=NSLOCTEXT(\"[212C611E4063DCDEF7B57583D9CD9BF2]\", \"E04F2E8742E7BCC94BEED4830519CFD4\", \"None\"),isStackable_7_62B26FAB4BC04A706C722797E3C992CE=True,thumbnail_9_67725CD9403BEA07F5C2CDA30062DCF3=None,Class_12_AF1AF12A4F0498BC96E161BF73632AA2=None,MaxStack_15_D7DF4220481B8B4473C4A2BEC01741EB=0)")) ContentToAdd))