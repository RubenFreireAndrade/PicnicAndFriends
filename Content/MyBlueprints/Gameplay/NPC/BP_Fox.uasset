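; BP_Fox is an interactable NPC that shows dialogue to the third-person player character.
; Entering its InteractTrigger creates a DialogueBox widget on screen, and leaving removes it.
; NPCInteract passes NpcText to the widget, then either removes it or updates its TextIndex, based on comparing text length with that index.
; A DoOnce gates each interaction and is re-armed through ResetDialogue on both branches.
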(event OnComponentBeginOverlap(InteractTrigger)
  (params (OverlappedComponent :type Primitive%20Component%20Object%20Reference) (OtherActor :type Actor%20Object%20Reference) (OtherComp :type Primitive%20Component%20Object%20Reference) (OtherBodyIndex :type Integer) (bFromSweep :type Boolean) (SweepResult :type Hit%20Result%20Structure%20%28by%20ref%29))
  (Utilities|Casting|CastToBP_ThirdPersonCharacter OtherActor)
  (bind _returnvalue (UserInterface|CreateWidget "/Game/MyBlueprints/Gameplay/NPC/DialogueBox.DialogueBox_C"))
  (bind _output_get (Variables|Default|SetDialogueUI _returnvalue))
  (UserInterface|Viewport|AddtoViewport _output_get 0))

(event OnComponentEndOverlap(InteractTrigger)
  (params (OverlappedComponent :type Primitive%20Component%20Object%20Reference) (OtherActor :type Actor%20Object%20Reference) (OtherComp :type Primitive%20Component%20Object%20Reference) (OtherBodyIndex :type Integer))
  (bind _dialogueui (Variables|Default|GetDialogueUI))
  (Utilities|Casting|CastToBP_ThirdPersonCharacter OtherActor)
  (Utilities|IsValid _dialogueui
    (:Is%20Valid
      (Widget|RemovefromParent _dialogueui))))

(event Custom|ResetDialogue
  (bind _dialogueui (Variables|Default|GetDialogueUI))
  (bind _npctext (Variables|Default|GetNpcText))
  (bind _returnvalue (Utilities|Array|Length _npctext))
  (bind _returnvalue_2 (+ _returnvalue 1))
  (Utilities|FlowControl|DoOnce false) ; enters at Reset
)

(event EventNPCInteract
  (bind _dialogueui (Variables|Default|GetDialogueUI))
  (bind _npctext (Variables|Default|GetNpcText))
  (bind _returnvalue (Utilities|Array|Length _npctext))
  (bind _returnvalue_2 (+ _returnvalue 1))
  (Development|PrintString "Interacting")
  (Utilities|FlowControl|DoOnce false
    (:Completed
      (Variables|/Game/MyBlueprints/Gameplay/NPC/DialogueBox.DialogueBox_C|SetText _dialogueui (Variables|Default|GetNpcText))
      (Widget|SetVisibility (Variables|/Game/MyBlueprints/Gameplay/NPC/DialogueBox.DialogueBox_C|GetNpcText _dialogueui) "Visible")
      (if (> _returnvalue_2 (- (Variables|/Game/MyBlueprints/Gameplay/NPC/DialogueBox.DialogueBox_C|GetTextIndex (Variables|Default|GetDialogueUI)) 1))
        (Widget|RemovefromParent (Variables|Default|GetDialogueUI))
        (CallFunction|ResetDialogue)
        (else
          (Variables|/Game/MyBlueprints/Gameplay/NPC/DialogueBox.DialogueBox_C|SetTextIndex (Variables|Default|GetDialogueUI) _returnvalue_2)
          (CallFunction|ResetDialogue))))))

(fn ConstructionScript)