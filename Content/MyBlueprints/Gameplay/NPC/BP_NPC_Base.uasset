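; BP_NPC_Base is a base NPC actor that shows its dialogue lines one at a time on interaction.
; Each NPCInteract event advances TextIndex through NpcText, lazily creating a DialogueBox widget and hiding it after the last line.
; Leaving InteractTrigger as the third-person character hides the dialogue and resets the index; entering only performs a cast.
; Leftover test logic is disconnected and never runs.
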(event OnComponentBeginOverlap(InteractTrigger)
  (params (OverlappedComponent :type Primitive%20Component%20Object%20Reference) (OtherActor :type Actor%20Object%20Reference) (OtherComp :type Primitive%20Component%20Object%20Reference) (OtherBodyIndex :type Integer) (bFromSweep :type Boolean) (SweepResult :type Hit%20Result%20Structure%20%28by%20ref%29))
  (Utilities|Casting|CastToBP_ThirdPersonCharacter OtherActor))

(event OnComponentEndOverlap(InteractTrigger)
  (params (OverlappedComponent :type Primitive%20Component%20Object%20Reference) (OtherActor :type Actor%20Object%20Reference) (OtherComp :type Primitive%20Component%20Object%20Reference) (OtherBodyIndex :type Integer))
  (bind _dialogueui (Variables|Default|GetDialogueUI))
  (Utilities|Casting|CastToBP_ThirdPersonCharacter OtherActor)
  (Utilities|IsValid _dialogueui
    (:Is%20Valid
      (Widget|SetVisibility _dialogueui "Hidden")
      (Variables|Default|SetTextIndex -1))))

(event EventNPCInteract
  (Development|PrintString "Interacting")
  (Math|Integer|IncrementInt (Variables|Default|GetTextIndex)
    (:%20%20
      (if (< (Variables|Default|GetTextIndex) (Utilities|Array|Length (Variables|Default|GetNpcText)))
        (Variables|Default|GetDialogueUI
          (:then
            _)
          (:else
            (bind _returnvalue (UserInterface|CreateWidget "/Game/MyBlueprints/Gameplay/NPC/DialogueBox.DialogueBox_C" (Game|GetPlayerController 0)))
            (bind _output_get (Variables|Default|SetDialogueUI _returnvalue))
            (UserInterface|Viewport|AddtoViewport _output_get 0)))
        (Rendering|Components|TextRender|SetText (Variables|/Game/MyBlueprints/Gameplay/NPC/DialogueBox.DialogueBox_C|GetNpcText (Variables|Default|GetDialogueUI)) (Utilities|Text|ToText(String) (Utilities|Array|Get(acopy) (Variables|Default|GetNpcText) (Variables|Default|GetTextIndex))))
        (Widget|SetVisibility (Variables|Default|GetDialogueUI) "Visible")
        (else
          (Widget|SetVisibility (Variables|Default|GetDialogueUI) "Hidden")
          (Variables|Default|SetTextIndex -1))))))

(fn ConstructionScript)